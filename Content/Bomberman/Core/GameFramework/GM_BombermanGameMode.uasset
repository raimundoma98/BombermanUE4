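; Bomberman game mode that manages the in-game HUD and the end-of-match screen.
; BeginPlay sets game-only input, shows the game widget and pre-creates the end-game widget.
; EndGame pauses, switches to UI input, swaps widgets, shows colored result text and binds the reset button to reload the current level.
; The logic filling both players' scores and colors is disconnected, so it never runs.
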(event Custom|RestartGame
  ;[1 1 1] Reset Game
  (bind _returnvalue (Game|GetCurrentLevelName true))
  (Game|OpenLevel(byName) (Utilities|String|StringToName _returnvalue)))

(event EventBeginPlay
  (bind _returnvalue (Game|GetPlayerController 0))
  ;[1 1 1] Create widgets and show Game widget
  (Input|SetInputModeGameOnly _returnvalue)
  (bind _returnvalue_2 (UserInterface|CreateWidget "/Game/Bomberman/UI/BP_GameWidget.BP_GameWidget_C" _returnvalue))
  (bind _output_get (Variables|Default|SetGameWidget _returnvalue_2))
  (Utilities|FlowControl|Sequence
    (:then_0
      (if (not (UserInterface|Viewport|IsinViewport _output_get))
        (UserInterface|Viewport|AddtoViewport _output_get 0)))
    (:then_1
      (bind _returnvalue_3 (UserInterface|CreateWidget "/Game/Bomberman/UI/BP_EndGameWidget.BP_EndGameWidget_C" _returnvalue))
      (Variables|Default|SetEndGameWidget _returnvalue_3))))

(event EventEndGame
  (params (ResultText :type String) (TextColor :type Linear%20Color%20Structure))
  (bind _returnvalue (Game|GetPlayerController 0))
  (bind _endgamewidget (Variables|Default|GetEndGameWidget))
  (bind _endgamewidget_2 (Variables|Default|GetEndGameWidget))
  ;[1 1 1] Show EndGame widget
  (Variables|/Script/Engine.PlayerController|SetbShowMouseCursor _returnvalue true)
  (Input|SetInputModeUIOnly _returnvalue 0 "DoNotLock")
  (Game|SetGamePaused true)
  (Widget|RemovefromParent (Variables|Default|GetGameWidget))
  (Rendering|Components|TextRender|SetText (Variables|/Script/Bomberman.EndGameWidget|GetResultText _endgamewidget) (Utilities|Text|ToText(String) ResultText))
  (Appearance|SetColorandOpacity (Variables|/Script/Bomberman.EndGameWidget|GetResultText _endgamewidget) (Utilities|Struct|MakeSlateColor TextColor) :!class /Script/UMG.TextBlock)
  (EventDispatchers|BindEventtoOnClicked (Variables|/Script/Bomberman.EndGameWidget|GetResetButton (Variables|Default|GetEndGameWidget)) (delegate Custom|RestartGame))
  (Utilities|FlowControl|Sequence
    (:then_0
      ;;[1 1 1] Set Score Text
      (bind _asbomberman_game_instance (Utilities|Casting|CastToBombermanGameInstance (Game|GetGameInstance))))
    (:then_1
      (if (not (UserInterface|Viewport|IsinViewport _endgamewidget_2))
        (UserInterface|Viewport|AddtoViewport _endgamewidget_2 0)))))

(fn ConstructionScript)