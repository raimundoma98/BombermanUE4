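; BP_BombermanCamera is the Bomberman game's camera actor, providing a timed screen shake effect.
; The ScreenShake event takes a duration and magnitude, stores the current location, and sets the timeline length to that duration.
; Each timeline update offsets the actor randomly in X and Y around that stored location, leaving Z unchanged, then restores it when finished.
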(event EventBeginPlay)

(event Collision|EventActorBeginOverlap
  (params (OtherActor :type Actor%20Object%20Reference)))

(event EventTick
  (params (DeltaSeconds :type Float%20%28single-precision%29)))

(event EventScreenShake
  (params (Duration :type Float%20%28single-precision%29) (Magnitude :type Float%20%28single-precision%29))
  ;[1 1 1] ScreenShake Animation
  (Components|Timeline|SetTimelineLength (Variables|Default|GetScreenShakeAnimation) Duration)
  (Variables|Default|SetMagnitude Magnitude)
  (Variables|Default|SetInitialLocation (Transformation|GetActorLocation))
  (Timeline|ScreenShakeAnimation PlayFromStart
    (:Update
      (Utilities|FlowControl|Sequence
        (:then_0
          (Variables|Default|SetX (* (Math|Random|RandomFloatinRange -1.0 1.0) (Variables|Default|GetMagnitude))))
        (:then_1
          (Variables|Default|SetY (* (Math|Random|RandomFloatinRange -1.0 1.0) (Variables|Default|GetMagnitude))))
        (:then_2
          (Transformation|SetActorLocation (Math|Vector|MakeVector (+ (Variables|Default|GetX) (.X (Math|Vector|BreakVector (Variables|Default|GetInitialLocation)))) (+ (Variables|Default|GetY) (.Y (Math|Vector|BreakVector (Variables|Default|GetInitialLocation)))) (.Z (Math|Vector|BreakVector (Variables|Default|GetInitialLocation)))) false false))))
    (:Finished
      (Transformation|SetActorLocation (Variables|Default|GetInitialLocation) false false))))

(fn ConstructionScript)